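; Player controller for the TTRPG game that handles click-to-move and mouse-wheel camera zoom on BP_PlayerHero through Enhanced Input.
; Holding follows the cursor, while short presses call MoveTo, which validates the destination with an overlap box.
; Validation samples random navmesh points, redirecting clicks on interactables to the sampled spot nearest the hero.
; MoveTo and EndMoveTo notify the game mode; Tick's PawnMovementStop check is disconnected.
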(event Input|EnhancedActionEvents|EnhancedInputActionin_ScaleCamera
  (params (ActionValue :type Vector%202D%20Structure) (ElapsedSeconds :type Float%20%28double-precision%29) (TriggeredSeconds :type Float%20%28double-precision%29) (InputAction :type Input%20Action%20Object%20Reference :default "/Game/TTRPG/Input/in_ScaleCamera.in_ScaleCamera"))
  (bind _x (Math|Vector2D|BreakVector2D ActionValue))
  ;[1 1 1] Scale Camera
  (Development|PrintString (Utilities|String|Append "Wheel Scrolled with Value of: " (Utilities|String|ToString(Float) _x)) false false)
  (bind _returnvalue (Actor|GetActorOfClass "/Game/TTRPG/Blueprints/BP_PlayerHero.BP_PlayerHero_C"))
  (Default|AdjustSpringArm _returnvalue _x))

(event Input|EnhancedActionEvents|EnhancedInputActionin_MouseClick
  (params (ActionValue :type Boolean) (ElapsedSeconds :type Float%20%28double-precision%29) (TriggeredSeconds :type Float%20%28double-precision%29) (InputAction :type Input%20Action%20Object%20Reference :default "/Game/TTRPG/Input/in_MouseClick.in_MouseClick"))
  (bind (_hit _location) (CallFunction|GetLocationUnderCursor))
  (:Triggered
    (if _hit
      (bind _output_get (Variables|Default|SetCachedDestination _location))
      (CallFunction|Follow _output_get)))
  (:Started
    (AI|Navigation|StopMovement))
  (:Ongoing
    (if (< ElapsedSeconds (Variables|Default|GetPressedThreshold)) :!label _label
      (CallFunction|Moveto (Variables|Default|GetCachedDestination))))
  (:Canceled
    (goto _label)))

(event EventBeginPlay
  (bind _returnvalue (PlayerController|LocalPlayerSubsystems|GetEnhancedInputLocalPlayerSubsystem))
  (Utilities|IsValid _returnvalue
    (:Is%20Valid
      (Input|AddMappingContext _returnvalue "/Game/TTRPG/Input/MouseandKeyboard.MouseandKeyboard" 1 "(bIgnoreAllPressedKeysUntilRelease=True,bForceImmediately=False,bNotifyUserSettings=False)")
      (bind _asbp_player_hero (Utilities|Casting|CastToBP_PlayerHero (Pawn|GetControlledPawn)))
      (bind _output_get (Variables|Default|SetcontrolledPlayerHero _asbp_player_hero))
      (Variables|/Script/Engine.CharacterMovementComponent|SetMaxWalkSpeed (Variables|/Script/Engine.Character|GetCharacterMovement _output_get) (Variables|Default|GetplayerMaxSpeed)))))

(event EventTick
  (params (DeltaSeconds :type Float%20%28single-precision%29))
  (if (Variables|Default|GetisMoving)
    (CallFunction|PawnMovementStop)))

(fn ConstructionScript
  (|CallParentFunction))

(fn Moveto
  (params (Location :type Vector :default "0, 0, 0"))
  (bind _playermovebox (Variables|Default|GetPlayerMoveBox))
  (Development|PrintString "Began Custom Move To" false false)
  (Variables|Default|SetisMoving true)
  (Transformation|SetWorldLocation _playermovebox Location false false)
  (bind (_boolvalid _vectorlocation) (CallFunction|ValidateDestinationClick _playermovebox Location))
  (Development|PrintString (Utilities|String|Append "Custom Moving To " (Utilities|String|ToString(Vector) _vectorlocation)))
  (if _boolvalid
    (bind _asttrpg_base (Utilities|Casting|CastToTTRPG_Base (Game|GetGameMode)))
    (Default|CharacterBeganMoving _asttrpg_base)
    (|CallParentFunction _vectorlocation)
    (bind _asttrpg_base_2 (Utilities|Casting|CastToTTRPG_Base (Game|GetGameMode)))
    (bind _asbp_player_hero (Utilities|Casting|CastToBP_PlayerHero (Pawn|GetControlledPawn)))
    (Default|ResetSpringArm _asbp_player_hero)
    (else
      (Development|PrintString "Not A Valid Move Location; Canceling Move"))))

(fn PawnMovementStop)

(fn EndMoveto
  (Development|PrintString "Controller: Ending Moving")
  (Variables|Default|SetisMoving false)
  (bind _asttrpg_base (Utilities|Casting|CastToTTRPG_Base (Game|GetGameMode)))
  (Default|CharacterEndMoving _asttrpg_base))

(fn SetPlayerSpeed
  (params (NewParam :type Float%20%28double-precision%29))
  (Variables|/Script/Engine.CharacterMovementComponent|SetMaxWalkSpeed (Variables|/Script/Engine.Character|GetCharacterMovement (Variables|Default|GetcontrolledPlayerHero)) NewParam)
  (Development|PrintString "Speed Updated"))

(fn ValidateDestinationClick
  (params (destinationbox :type Box%20Component%20Object%20Reference) (inVectorLocation :type Vector))
  (bind _overlappingactors (Collision|GetOverlappingActors destinationbox "/Game/TTRPG/Blueprints/InteractableObject.InteractableObject_C" :!class /Script/Engine.PrimitiveComponent))
  (bind _z (Math|Vector|BreakVector inVectorLocation))
  (bind _output (Utilities|Array|Get(acopy) _overlappingactors))
  (bind _returnvalue (Transformation|GetActorLocation _output))
  (bind (_x _y) (Math|Vector|BreakVector _returnvalue))
  (bind _returnvalue_2 (Math|Vector|MakeVector _x _y _z))
  (Development|PrintString (Utilities|String|Append "Move Vector Before Validation " (Utilities|String|ToString(Vector) inVectorLocation)))
  (if (Utilities|Array|IsNotEmpty _overlappingactors)
    (Development|PrintString "Overlapping true" false)
    (bind (_vectrandomspot _boolvalid) (CallFunction|GetClosestPoint _returnvalue_2))
    (if _boolvalid
      (Development|PrintString "Succeed Random Point Pick")
      (return true _vectrandomspot)
      (else
        (Development|PrintString "Failed Random Point Pick")
        (return false _returnvalue_2)))
    (else
      (bind _boolvalid_2 (CallFunction|GetClosestPoint inVectorLocation))
      (if _boolvalid_2 ; Validate if point is within nav mesh before moving there
        (return true inVectorLocation)
        (else
          (return false inVectorLocation))))))

(fn GetClosestPoint
  (params (vectOrigin :type Vector))
  (while (<= (LocalVariables|GetintWhileLoopIterator) (LocalVariables|GetintNumberOfAttempts))
    (bind (_randomlocation _returnvalue) (Class|NavigationSystemV1|GetRandomLocationinNavigableRadius vectOrigin 5e+01 0 0))
    (if _returnvalue
      (if (> (LocalVariables|GettempSmallestDistance) (Math|Vector|Distance(Vector) _randomlocation (Transformation|GetActorLocation (Variables|Default|GetcontrolledPlayerHero))))
        (LocalVariables|SettempSmallestDistance (Math|Vector|Distance(Vector) _randomlocation (Transformation|GetActorLocation (Variables|Default|GetcontrolledPlayerHero))))
        (LocalVariables|SettempBoolReturn true)
        (LocalVariables|SetvecTempClosestVector _randomlocation)))
    (LocalVariables|SetintWhileLoopIterator (+ (LocalVariables|GetintWhileLoopIterator) 1)))
  (return (LocalVariables|GetvecTempClosestVector) (LocalVariables|GettempBoolReturn)))