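; Quest controller for a Shire-set tabletop RPG project that stores active quests and tracks their step progress.
; BeginPlay fills CurrentQuests with two hardcoded quests, a test quest and "Off Into The Blue", built from nested requirement structs.
; ProgressQuest flags a requirement complete, then advances CurrentStep if a shared bool, never reset here, survives checking that step's requirements.
; The node marking a whole quest completed is unconnected.
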(event EventBeginPlay
  (CallFunction|GenerateTestQuest)
  (CallFunction|GenerateQuest))

(event EventTick
  (params (DeltaSeconds :type Float%20%28single-precision%29)))

(fn GenerateTestQuest
  (bind _output_get (LocalVariables|SettempQuestVariable (Utilities|Struct|MakeQuest "quest_TestQuest1" "This is a test quest." "The purpose of this quest is to test the functionality of quests without having to handle the JSON serializations" (Utilities|Array|MakeArray (Utilities|Struct|MakeQuestRequirement "requirement_TestRequirement1" "Test Requirement 1" 1 false) (Utilities|Struct|MakeQuestRequirement "requirement_TestRequirement2" "Test Requirement 2" 2 false)))))
  (Utilities|Array|Add (Variables|Default|GetcurrentQuests) _output_get)
  (Development|PrintString "Test Quest Added to Controller"))

(fn GenerateQuest
  (bind _questrequirement (Utilities|Struct|MakeQuestRequirement "requirement_Conspiracy1_VisitOverhill" "Go North To Overhill" 2 false))
  (bind _questrequirement_2 (Utilities|Struct|MakeQuestRequirement "requirement_Conspiracy1_TalkToBilbo" "Go to Bag End and speak with Bilbo" 1 false))
  (bind _questrequirement_3 (Utilities|Struct|MakeQuestRequirement "requirement_Conspiracy1_CrossRiver" "Cross the River West of Overhill" 3 false))
  (bind _array (Utilities|Array|MakeArray _questrequirement_2 _questrequirement _questrequirement_3))
  (bind _quest (Utilities|Struct|MakeQuest "quest_Conspiracy1_OffIntoTheBlue" "Off Into The Blue" "Mr. Baggins sends the adventurers to Michel Delving to retrieve a map of the shire once belonging to The Old Took. This quest consists of part 1 of the overal Conspiracy Most Cracked." _array false 4))
  (bind _output_get (LocalVariables|SettempQuestVariable _quest))
  (Utilities|Array|Add (Variables|Default|GetcurrentQuests) _output_get)
  (Development|PrintString (Utilities|String|Append (.InternalQuestName (Utilities|Struct|BreakQuest _quest)) " Added to Quest Controller") false false))

(fn ProgressQuest
  (params (QuestToProgress :type Integer) (Requirement%20to%20Complete :type Integer))
  (bind _currentquests (Variables|Default|GetcurrentQuests))
  (bind _output (Utilities|Array|Get(acopy) _currentquests QuestToProgress))
  (bind (_internalquestname _questdisplayname _questdescription _questreqirements _completed _currentstep) (Utilities|Struct|BreakQuest _output))
  (Development|PrintString (Utilities|String|Append "Progressing Quest: " (Utilities|String|ToString(Integer) Requirement%20to%20Complete)) false)
  (if (> Requirement%20to%20Complete -1) ; If we are NOT progressing a requirement, complete the quest
    (Development|PrintString "Has dependant requirement" false)
    (Utilities|Struct|SetmembersinQuestRequirement (Utilities|Array|Get(acopy) _questreqirements (- Requirement%20to%20Complete 1)) true)
    (bind _arrayelement (Utilities|ForEachLoopRef _questreqirements)
      (:LoopBody
        (Development|PrintString (Utilities|String|Append "Testing Requirement: " (.InternalRequirementName (Utilities|Struct|BreakQuestRequirement _arrayelement))) false)
        (if (LocalVariables|GetboolTempBool)
          (if (== (.RequirementStep (Utilities|Struct|BreakQuestRequirement _arrayelement)) _currentstep)
            (if (.CompletedFlag (Utilities|Struct|BreakQuestRequirement _arrayelement))
              (Development|PrintString (Utilities|String|Append (.InternalRequirementName (Utilities|Struct|BreakQuestRequirement _arrayelement)) " completed") false)
              (else
                (LocalVariables|SetboolTempBool false)))
            (else
              (Development|PrintString "Not In Current Step" false)))
          (else
            (Development|PrintString "Skipped because found a unfulfilled quest requirement already" false))))
      (:Completed
        (Development|PrintString (Utilities|String|Append "All Requirements For Step Met? " (Utilities|String|ToString(Boolean) (LocalVariables|GetboolTempBool))) false)
        (if (LocalVariables|GetboolTempBool) ; Check if every requirement for the current step is completed. Then Progress the quest
          (Utilities|Struct|SetmembersinQuest _output false (+ _currentstep 1))
          (if true
            _))))
    (else
      (Development|PrintString "Does not have dependent requirements" false))))