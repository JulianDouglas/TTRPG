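; BP_SoundController is a sound controller Blueprint in the TTRPG project that plays non-spatial one-shot sounds, including page turns.
; PlaySoundOnce prints the name of the passed sound and plays it in 2D, while PlayPageTurnSound picks a random entry from the PageTurnSounds array.
; Both events randomize the pitch around normal on each play to vary repeated sounds.
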(event Custom|PlaySoundOnce
  (params (Sound%20to%20play%20once :type Sound%20Wave%20Object%20Reference))
  (Development|PrintString (Utilities|String|Append "Playing sound " (Utilities|GetDisplayName Sound%20to%20play%20once)) false)
  (Audio|PlaySound2D Sound%20to%20play%20once 1.0 (Math|Random|RandomFloatinRange 0.75 1.25) 0.0 0 0))

(event Custom|PlayPageTurnSound
  (bind _pageturnsounds (Variables|Default|GetPageTurnSounds))
  (Audio|PlaySound2D (Utilities|Array|Get(acopy) _pageturnsounds (Math|Conversions|ToInteger(Byte) (Class|KismetMathLibrary|RandomInteger64inRange 0 (Class|KismetMathLibrary|ToInt64(Integer) (- (Utilities|Array|Length _pageturnsounds) 1))))) 1.0 (Math|Random|RandomFloatinRange 0.75 1.25) 0.0 0 0))

(event EventBeginPlay)

(event EventTick
  (params (DeltaSeconds :type Float%20%28single-precision%29)))