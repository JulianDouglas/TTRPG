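; BP_CharacterSheet is a tabletop RPG character sheet that stores and looks up One Ring skills in a SkillList array of structs.
; SetSkillValue rebuilds the matching entry with a new value and favoured flag, keeps its category, and prints the result.
; GetSkillValue searches by skill name but uses the matched skill's Value as the array index for the name, favoured flag and value it returns.
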(fn SetSkillValue
  (params (SkillToSet :type Skills_OneRing_Roll%20Enum :default "NewEnumerator0") (Value :type Integer) (Favored :type Boolean))
  (Development|PrintString 0 (Utilities|String|Append "Setting Skill " (Utilities|String|EnumtoString SkillToSet) " to value " (Utilities|String|ToString(Integer) Value) " and favored is " (Utilities|String|ToString(Boolean) Favored)) false false)
  (for (_array_element _array_index) (Variables|Default|GetSkillList)
    (if (Utilities|Enum|Equal(Enum) (.SkillName (Utilities|Struct|BreakOneRing_Skills _array_element)) SkillToSet)
      (Utilities|Array|SetArrayElem (Variables|Default|GetSkillList) _array_index (Utilities|Struct|MakeOneRing_Skills (.SkillName (Utilities|Struct|BreakOneRing_Skills _array_element)) Value Favored (.Category (Utilities|Struct|BreakOneRing_Skills _array_element))))
      (LocalVariables|SettempArrayElement _array_index)))
  (Development|PrintString 0 (Utilities|String|Append (Utilities|String|EnumtoString (.skillname (Utilities|Array|Get(acopy) (Variables|Default|GetSkillList) (LocalVariables|GettempArrayElement)))) " is now " (Utilities|String|ToString(Integer) (.value (Utilities|Array|Get(acopy) (Variables|Default|GetSkillList) (LocalVariables|GettempArrayElement)))) " and favored is " (Utilities|String|ToString(Boolean) (.favouredskill (Utilities|Array|Get(acopy) (Variables|Default|GetSkillList) (LocalVariables|GettempArrayElement))))) false false)
  (return))

(fn GetSkillValue
  (params (Skill%20Name :type Skills_OneRing_Roll%20Enum :default "NewEnumerator0"))
  (Development|PrintString 0 (Utilities|String|EnumtoString Skill%20Name))
  (for _array_element (Variables|Default|GetSkillList)
    (if (Utilities|Enum|Equal(Enum) (.SkillName (Utilities|Struct|BreakOneRing_Skills _array_element)) Skill%20Name)
      (LocalVariables|SettempArrayValue (.Value (Utilities|Struct|BreakOneRing_Skills _array_element)))))
  (return (Utilities|String|EnumtoString (.skillname (Utilities|Array|Get(acopy) (Variables|Default|GetSkillList) (LocalVariables|GettempArrayValue)))) (.favouredskill (Utilities|Array|Get(acopy) (Variables|Default|GetSkillList) (LocalVariables|GettempArrayValue))) (.value (Utilities|Array|Get(acopy) (Variables|Default|GetSkillList) (LocalVariables|GettempArrayValue)))))