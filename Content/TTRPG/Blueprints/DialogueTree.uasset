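; Dialogue tree component for interactable objects that runs branching conversations in the TTRPG game mode through an InteractableMenu widget.
; DisplayNode fills the page and builds response buttons, filtered by quest state and roll availability.
; Response checks can progress quests, teleport the hero, deactivate the dialogue, or roll One Ring skill checks that pick the next node by success degree.
; Gandalf runes upgrade results, and limited rolls disable themselves after use.
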(event EventBeginPlay
  (bind _asinteractable_object (Utilities|Casting|CastToInteractableObject (Components|GetOwner)))
  (Variables|Default|SetOwningInteractableObject _asinteractable_object))

(event EventTick
  (params (DeltaSeconds :type Float%20%28single-precision%29)))

(fn DisplayNode
  (params (nodeToDisplay :type Integer))
  (Variables|Default|SetcurrentConverstaionNode nodeToDisplay)
  ;[1 1 1] Remove all current items
  (Widget|Panel|ClearChildren (Variables|/Game/TTRPG/UI/InteractableMenu.InteractableMenu_C|GetResponseBox (Variables|Default|GetinteractableMenu)))
  ;[1 1 1] Must Display Main Text and Title
  (Variables|/Script/UMG.TextBlock|SetText (Variables|/Game/TTRPG/UI/InteractableMenu.InteractableMenu_C|GetPageText (Variables|Default|GetinteractableMenu)) (Utilities|Text|ToText(String) (.optiontext (Utilities|Array|Get(acopy) (Variables|Default|GetConversationNodes) (Variables|Default|GetcurrentConverstaionNode)))))
  (Variables|/Script/UMG.TextBlock|SetText (Variables|/Game/TTRPG/UI/InteractableMenu.InteractableMenu_C|GetTitleText (Variables|Default|GetinteractableMenu)) (Utilities|Text|ToText(String) (.pagetitle (Utilities|Array|Get(acopy) (Variables|Default|GetConversationNodes) (Variables|Default|GetcurrentConverstaionNode)))))
  (Class|Image|SetBrush (Variables|/Game/TTRPG/UI/InteractableMenu.InteractableMenu_C|GetPageImage (Variables|Default|GetinteractableMenu)) (Utilities|Struct|MakeSlateBrush (.DrawAs (Utilities|Struct|BreakSlateBrush (Variables|/Script/UMG.Image|GetBrush (Variables|/Game/TTRPG/UI/InteractableMenu.InteractableMenu_C|GetPageImage (Variables|Default|GetinteractableMenu))))) (.Tiling (Utilities|Struct|BreakSlateBrush (Variables|/Script/UMG.Image|GetBrush (Variables|/Game/TTRPG/UI/InteractableMenu.InteractableMenu_C|GetPageImage (Variables|Default|GetinteractableMenu))))) (.Mirroring (Utilities|Struct|BreakSlateBrush (Variables|/Script/UMG.Image|GetBrush (Variables|/Game/TTRPG/UI/InteractableMenu.InteractableMenu_C|GetPageImage (Variables|Default|GetinteractableMenu))))) (.ImageSize (Utilities|Struct|BreakSlateBrush (Variables|/Script/UMG.Image|GetBrush (Variables|/Game/TTRPG/UI/InteractableMenu.InteractableMenu_C|GetPageImage (Variables|Default|GetinteractableMenu))))) (.Margin (Utilities|Struct|BreakSlateBrush (Variables|/Script/UMG.Image|GetBrush (Variables|/Game/TTRPG/UI/InteractableMenu.InteractableMenu_C|GetPageImage (Variables|Default|GetinteractableMenu))))) (.TintColor (Utilities|Struct|BreakSlateBrush (Variables|/Script/UMG.Image|GetBrush (Variables|/Game/TTRPG/UI/InteractableMenu.InteractableMenu_C|GetPageImage (Variables|Default|GetinteractableMenu))))) (.OutlineSettings (Utilities|Struct|BreakSlateBrush (Variables|/Script/UMG.Image|GetBrush (Variables|/Game/TTRPG/UI/InteractableMenu.InteractableMenu_C|GetPageImage (Variables|Default|GetinteractableMenu))))) (.pageimage (Utilities|Array|Get(acopy) (Variables|Default|GetConversationNodes) (Variables|Default|GetcurrentConverstaionNode)))))
  ;[1 1 1] Toggle Default Response
  (if (Utilities|Array|IsEmpty (.responses (Utilities|Array|Get(acopy) (Variables|Default|GetConversationNodes) (Variables|Default|GetcurrentConverstaionNode))))
    (Development|PrintString "Response Empty" false)
    (Default|ToggleDefaultOption (Variables|Default|GetinteractableMenu) true)
    (else
      (Development|PrintString "Responses Exist" false)
      (Default|ToggleDefaultOption (Variables|Default|GetinteractableMenu) false)
      (Widget|Panel|AddChild (Variables|/Game/TTRPG/UI/InteractableMenu.InteractableMenu_C|GetResponseBox (Variables|Default|GetinteractableMenu)) (Variables|Default|GetspacerObject))
      ;[1 1 1] Then Loop through response buttons
      (for (_array_element _array_index) (.responses (Utilities|Array|Get(acopy) (Variables|Default|GetConversationNodes) (Variables|Default|GetcurrentConverstaionNode)))
        (bind _todisplay (CallFunction|ValidateResponse _array_element))
        (if _todisplay
          (bind _returnvalue (UserInterface|CreateWidget "/Game/TTRPG/UI/responseButton.responseButton_C" (Game|GetPlayerController 0)))
          (if (.RequiresRoll (Utilities|Struct|BreakDialogueResponses _array_element))
            (Variables|/Script/UMG.TextBlock|SetText (Variables|/Game/TTRPG/UI/responseButton.responseButton_C|GetTextBlock_0 _returnvalue) (Utilities|Text|ToText(String) (Utilities|String|Append "(" (Utilities|String|EnumtoString (.rollSkillToRoll (Utilities|Struct|BreakDialogueResponses _array_element))) ") " (.ResponseText (Utilities|Struct|BreakDialogueResponses _array_element)))))
            (else
              (Variables|/Script/UMG.TextBlock|SetText (Variables|/Game/TTRPG/UI/responseButton.responseButton_C|GetTextBlock_0 _returnvalue) (Utilities|Text|ToText(String) (.ResponseText (Utilities|Struct|BreakDialogueResponses _array_element))))))
          (Variables|/Game/TTRPG/UI/responseButton.responseButton_C|SetnextNode _returnvalue (.ResponseDestination (Utilities|Struct|BreakDialogueResponses _array_element)))
          (Variables|/Game/TTRPG/UI/responseButton.responseButton_C|SetinteractableMenu _returnvalue (Variables|Default|GetinteractableMenu))
          (Variables|/Game/TTRPG/UI/responseButton.responseButton_C|SetexitBoolean _returnvalue (.QuitsDialogue (Utilities|Struct|BreakDialogueResponses _array_element)))
          (Variables|/Game/TTRPG/UI/responseButton.responseButton_C|SetcurrentNode _returnvalue _array_index)
          (Widget|Panel|AddChild (Variables|/Game/TTRPG/UI/InteractableMenu.InteractableMenu_C|GetResponseBox (Variables|Default|GetinteractableMenu)) _returnvalue))))))

(fn BeginDialogue
  (bind _returnvalue (Game|GetPlayerController 0))
  (bind _asttrpg_base (Utilities|Casting|CastToTTRPG_Base (Game|GetGameMode))
    (:then
      (Variables|/Game/TTRPG/TTRPG_Base.TTRPG_Base_C|SetboolInDialogue _asttrpg_base true)
      (bind _returnvalue_2 (UserInterface|CreateWidget "/Game/TTRPG/UI/InteractableMenu.InteractableMenu_C" _returnvalue))
      (Variables|/Game/TTRPG/UI/InteractableMenu.InteractableMenu_C|SetOwningDialogueTree _returnvalue_2 self)
      (Variables|Default|SetinteractableMenu _returnvalue_2)
      (Variables|Default|SetspacerObject (Class|PanelWidget|GetChildat (Variables|/Game/TTRPG/UI/InteractableMenu.InteractableMenu_C|GetResponseBox _returnvalue_2)))
      (CallFunction|DisplayNode)
      (UserInterface|Viewport|AddtoViewport _returnvalue_2 1)
      (Input|SetInputModeUIOnly _returnvalue _returnvalue_2 "DoNotLock" false))
    (:CastFailed
      (Development|PrintString "Game Mode Not TTRPG" false))))

(fn EndDialogue
  (params (interactableMenuUI :type Interactable%20Menu%20Object%20Reference))
  (Development|PrintString "Ended Dialogue" false)
  (Class|GameViewportSubsystem|RemoveWidget (|GameViewportSubsystem) interactableMenuUI)
  (Input|SetInputModeGameandUI (Game|GetPlayerController 0) 0 "DoNotLock" true false)
  (bind _asttrpg_base (Utilities|Casting|CastToTTRPG_Base (Game|GetGameMode)))
  (Variables|/Game/TTRPG/TTRPG_Base.TTRPG_Base_C|SetboolInDialogue _asttrpg_base false)
  (Default|ReTriggerInteractableObjectOverlap _asttrpg_base))

(fn GetCurrentMainText
  (return (.optiontext (Utilities|Array|Get(acopy) (Variables|Default|GetConversationNodes) (Variables|Default|GetcurrentConverstaionNode)))))

(fn ValidateResponse
  (params (Response%20To%20Display :type Dialogue%20Responses%20Structure))
  (bind (_responsetext _responsedestination _requiresroll _rollactive _rollskilltoroll _rollsuccessdestination _rollgreatsuccessdestination _rollextraordinarysuccessdestination _rollfailuredestination _rollbestperson _rolllimittoone _quitsdialogue _destinationdialoguetree _deactivatesdialogue _incrementsquest _questtoincrement _requriementtocomplete _requirequest _questtorequire _steptorequire) (Utilities|Struct|BreakDialogueResponses Response%20To%20Display))
  (if _requirequest
    (bind _asttrpg_base (Utilities|Casting|CastToTTRPG_Base (Game|GetGameMode)))
    (for _array_element (Variables|/Game/TTRPG/Blueprints/Code-Implimented-Blueprints/BP_QuestController.BP_QuestController_C|GetcurrentQuests (Actor|GetComponentbyClass _asttrpg_base "/Game/TTRPG/Blueprints/Code-Implimented-Blueprints/BP_QuestController.BP_QuestController_C"))
      (if (Utilities|Enum|Equal(Enum) (.InternalQuestName (Utilities|Struct|BreakQuest _array_element)) _questtorequire) ; Display Response only if the required quest is active
        (if (.Completed (Utilities|Struct|BreakQuest _array_element)) ; Display Response only if the required quest is not completed
          (LocalVariables|SettempDisplayCondition false :!label _label)
          (else
            (if (Utilities|Array|IsNotEmpty _steptorequire) ; Display only if on the accepted step or the Step Requirements is empty
              (if (Utilities|Array|ContainsItem _steptorequire (.CurrentStep (Utilities|Struct|BreakQuest _array_element)))
                _
                (else
                  (Development|PrintString "Required Step does NOT contain current Step")
                  (goto _label))))
            (LocalVariables|SettempDisplayCondition true)))
        (else
          (goto _label)))))
  (if _requiresroll
    (if _rollactive ; Only display response if rollActive is valid
      _
      (else
        (LocalVariables|SettempDisplayCondition false))))
  (Development|PrintString (Utilities|String|ToString(Boolean) (LocalVariables|GettempDisplayCondition)) false)
  (return (LocalVariables|GettempDisplayCondition)))

(fn IncrementCheck
  (params (currentNode :type Integer))
  (bind _conversationnodes (Variables|Default|GetConversationNodes))
  (bind _currentconverstaionnode (Variables|Default|GetcurrentConverstaionNode))
  (bind _output (Utilities|Array|Get(acopy) _conversationnodes _currentconverstaionnode))
  (bind _output_2 (Utilities|Array|Get(acopy) (.responses _output) currentNode))
  (if (.incrementsquest _output_2)
    (bind _asttrpg_base (Utilities|Casting|CastToTTRPG_Base (Game|GetGameMode)))
    (for (_array_element _array_index) (Variables|/Game/TTRPG/Blueprints/Code-Implimented-Blueprints/BP_QuestController.BP_QuestController_C|GetcurrentQuests (Variables|/Game/TTRPG/TTRPG_Base.TTRPG_Base_C|GetQuestController _asttrpg_base))
      (if (Utilities|Enum|Equal(Enum) (.InternalQuestName (Utilities|Struct|BreakQuest _array_element)) (.questtoincrement _output_2))
        (if (Utilities|Array|IsEmpty (.requriementtocomplete _output_2))
          (Development|PrintString "Prog w/o requirement" false)
          (Default|ProgressQuest (Variables|/Game/TTRPG/TTRPG_Base.TTRPG_Base_C|GetQuestController _asttrpg_base) _array_index -1)
          (else
            (Development|PrintString "Prog w/ requirement" false)
            (Default|ProgressQuest (Variables|/Game/TTRPG/TTRPG_Base.TTRPG_Base_C|GetQuestController _asttrpg_base) _array_index (.CurrentStep (Utilities|Struct|BreakQuest _array_element)))))))
    (else
      (Development|PrintString "Response does not increment quest" false))))

(fn RollResponseCheck
  (params (CurrentNode :type Integer) (NextNode :type Integer%20%28by%20ref%29))
  (bind _conversationnodes (Variables|Default|GetConversationNodes))
  (bind _currentconverstaionnode (Variables|Default|GetcurrentConverstaionNode))
  (bind _output (Utilities|Array|Get(acopy) _conversationnodes _currentconverstaionnode))
  (bind _output_2 (Utilities|Array|Get(acopy) (.responses _output) CurrentNode))
  (Utilities|String|LogString "Roll Response Check")
  (if (.requiresroll _output_2)
    (if (.rollactive _output_2)
      (bind _asttrpg_base (Utilities|Casting|CastToTTRPG_Base (Game|GetGameMode))
        (:then
          (bind (_success _failure _successdegree _gandalfrune _eyeofsauron) (Default|MakeSkillCheckOneRing _asttrpg_base (.rollskilltoroll _output_2) false false (.rollbestperson _output_2)))
          (LocalVariables|SettempSuccessDegree _successdegree)
          (Development|PrintString (Utilities|String|Append "Roll Result:  Success-" (Utilities|String|ToString(Boolean) _success) " Failure- " (Utilities|String|ToString(Boolean) _failure) " Success Icons- " (Utilities|String|EnumtoString _successdegree) " Gandalf Rune-" (Utilities|String|ToString(Boolean) _gandalfrune) " Eye of Sauron-" (Utilities|String|ToString(Boolean) _eyeofsauron)) false)
          (if _success ; If successful, determine degree of success, otherwise head to fail destination
            (if _gandalfrune
              (if (< (LocalVariables|GettempSuccessDegree) 2)
                (LocalVariables|SettempSuccessDegree (Utilities|Enum|ByteToEnumOneRing_DegreesOfSuccess (+ (LocalVariables|GettempSuccessDegree) 1)))))
            (switch Utilities|FlowControl|Switch|SwitchonOneRing_DegreesOfSuccess (LocalVariables|GettempSuccessDegree)
              (:NewEnumerator0
                (|SetBy-RefVar NextNode (.rollsuccessdestination _output_2) :!label _label))
              (:NewEnumerator1
                (|SetBy-RefVar NextNode (.rollgreatsuccessdestination _output_2)))
              (:NewEnumerator2
                (|SetBy-RefVar NextNode (.rollextraordinarysuccessdestination _output_2))))
            (elif _gandalfrune
              (goto _label)
              (else
                (|SetBy-RefVar NextNode (.rollfailuredestination _output_2)))))
          (if (.rolllimittoone _output_2) ; Checks for roll limiting and adjusts active flag accordingly.
            (|SetBy-RefVar (.rollactive _output_2) false)))
        (:CastFailed
          (Development|PrintString "Failed Cast in Roll Response Check")))
      (else
        (return)))
    (else
      (return))))

(fn FinalDeactivateDialogueCheck
  (if (Variables|Default|GetendingDialogue)
    (Variables|Default|Setactive false)
    (else
      (Variables|Default|Setactive true)))
  (Development|PrintString (Utilities|String|Append "Setting active flag for dialogue to " (Utilities|String|ToString(Boolean) (Variables|Default|Getactive))) false)
  (return))

(fn DeactivateDialogueCheck
  (params (responseNode :type Integer))
  (if (.deactivatesdialogue (Utilities|Array|Get(acopy) (.responses (Utilities|Array|Get(acopy) (Variables|Default|GetConversationNodes) (Variables|Default|GetcurrentConverstaionNode))) responseNode))
    (Utilities|String|LogString "Setting Ending Dialogue Flag")
    (Variables|Default|SetendingDialogue true)))

(fn MovePlayerCheck
  (params (CurrentResponse :type Integer))
  (bind _conversationnodes (Variables|Default|GetConversationNodes))
  (bind _currentconverstaionnode (Variables|Default|GetcurrentConverstaionNode))
  (bind _output (Utilities|Array|Get(acopy) _conversationnodes _currentconverstaionnode))
  (bind _output_2 (Utilities|Array|Get(acopy) (.responses _output) CurrentResponse))
  (bind _location (Math|Transform|BreakTransform (.vectomovedest _output_2)))
  (bind (_x _y) (Math|Vector|BreakVector _location))
  (if (.boolmovescharacter _output_2)
    (bind _asttrpg_base_controller (Utilities|Casting|CastToTTRPG_BaseController (Game|GetPlayerController 0))
      (:then
        (Development|PrintString (Utilities|String|ToString(Transform) (Transformation|GetActorTransform (Variables|/Game/TTRPG/Blueprints/TTRPG_BaseController.TTRPG_BaseController_C|GetcontrolledPlayerHero _asttrpg_base_controller))))
        (Transformation|SetActorTransform (Variables|/Game/TTRPG/Blueprints/TTRPG_BaseController.TTRPG_BaseController_C|GetcontrolledPlayerHero _asttrpg_base_controller) (Math|Transform|MakeTransform (Math|Vector|MakeVector _x _y (.Z (Math|Vector|BreakVector (.Location (Math|Transform|BreakTransform (Transformation|GetActorTransform (Variables|/Game/TTRPG/Blueprints/TTRPG_BaseController.TTRPG_BaseController_C|GetcontrolledPlayerHero _asttrpg_base_controller))))))) (.Rotation (Math|Transform|BreakTransform (Transformation|GetActorTransform (Variables|/Game/TTRPG/Blueprints/TTRPG_BaseController.TTRPG_BaseController_C|GetcontrolledPlayerHero _asttrpg_base_controller)))) (.Scale (Math|Transform|BreakTransform (Transformation|GetActorTransform (Variables|/Game/TTRPG/Blueprints/TTRPG_BaseController.TTRPG_BaseController_C|GetcontrolledPlayerHero _asttrpg_base_controller))))) false true))
      (:CastFailed
        (Development|PrintString "Cast Failed in DialogueTree Move Player")))
    (else
      (return))))