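; Clickable TTRPG world object with an icon that outlines on hover and starts dialogue when the player is near.
; Click checks the player's collision box, then picks among active DialogueTree components, favouring active-quest matches, otherwise filtering by time of day and lowest priority value.
; Scale events show or hide the icon through interpolation on Tick, optionally gating display on quest step.
; Quest and time state come from the TTRPG_Base game mode.
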(event Custom|reScaleObject
  (Development|PrintString "Triggered RescaleObject Event" false)
  (if (Variables|Default|GetboolRequiresQuest)
    (bind _meetrequirement (CallFunction|VerifyQuestRequirement))
    (if _meetrequirement
      (Variables|Default|SettargetScaleVector (Variables|Default|GetresetScaleVector) :!label _label)
      (Variables|Default|Setbool_WithinPlayerRange true))
    (else
      (goto _label))))

(event Custom|OnBeginCursorOver_Event
  (params (TouchedActor :type Actor%20Object%20Reference))
  (Development|PrintString "Mouse Over event Triggered")
  (Rendering|SetRenderCustomDepth (Variables|Default|GetIcon) true))

(event Custom|OnEndCursorOver_Event
  (params (TouchedActor :type Actor%20Object%20Reference))
  (Rendering|SetRenderCustomDepth (Variables|Default|GetIcon) false))

(event Custom|ScaleInteractableObject
  (if (Variables|Default|GetboolRequiresQuest)
    (bind _meetrequirement (CallFunction|VerifyQuestRequirement))
    (if _meetrequirement
      (Variables|Default|SettargetScaleVector (Variables|Default|GetresetScaleVector) :!label _label)
      (Variables|Default|Setbool_WithinPlayerRange true))
    (else
      (goto _label))))

(event Custom|DownScaleInteractableObject
  (Variables|Default|SettargetScaleVector "0, 0, 0")
  (Variables|Default|Setbool_WithinPlayerRange false))

(event Custom|OnClick_Interact
  (params (TouchedActor :type Actor%20Object%20Reference) (ButtonPressed :type Key%20Structure :default "None"))
  (CallFunction|Interact (Variables|Default|GetPlayerInRange)))

(event EventBeginPlay
  (EventDispatchers|BindEventtoOnBeginCursorOver (delegate Custom|OnBeginCursorOver_Event))
  (Rendering|SetRenderCustomDepth (Variables|Default|GetIcon) false)
  (EventDispatchers|BindEventtoOnEndCursorOver (delegate Custom|OnEndCursorOver_Event))
  (EventDispatchers|BindEventtoOnClicked (delegate Custom|OnClick_Interact))
  (if (Utilities|Array|IsEmpty (Actor|GetComponentsByClass "/Game/TTRPG/Blueprints/DialogueTree.DialogueTree_C"))
    (Development|PrintString "Does not have Dialogue tree" false false)
    (else
      (Variables|Default|SetDialogueTree (Actor|GetComponentbyClass "/Game/TTRPG/Blueprints/DialogueTree.DialogueTree_C"))
      (Variables|Default|SethasDialogueTree true)
      (Development|PrintString "Set HasDialogue Tree Flag" false false)))
  (Variables|Default|SetresetScaleVector (Variables|/Script/Engine.SceneComponent|GetRelativeScale3D (Variables|Default|GetIcon))))

(event Collision|EventActorBeginOverlap
  (params (OtherActor :type Actor%20Object%20Reference))
  (bind _asbp_player_hero (Utilities|Casting|CastToBP_PlayerHero OtherActor)
    (:then
      (Variables|Default|SetPlayerInRange _asbp_player_hero)
      (Development|PrintString (Utilities|String|Append "Just Collided With: " (Variables|Default|GetObjectName)) false false)
      (if (Utilities|ClassIsChildOf (Utilities|GetClass OtherActor) "/Game/TTRPG/Blueprints/BP_PlayerHero.BP_PlayerHero_C")
        (Variables|Default|SetOverlappingPlayer true)))
    (:CastFailed
      (Development|PrintString "Overlapped Object Not Player" false))))

(event EventTick
  (params (DeltaSeconds :type Float%20%28single-precision%29))
  (CallFunction|ScaleObject DeltaSeconds false))

(event Collision|EventActorEndOverlap
  (params (OtherActor :type Actor%20Object%20Reference))
  (Utilities|Casting|CastToBP_PlayerHero OtherActor)
  (Development|PrintString "Player No Longer Overlapping" false)
  (Variables|Default|SetPlayerInRange 0)
  (if (Variables|Default|GetOverlappingPlayer)
    (Development|PrintString (Utilities|String|Append "No Longer Collided With: " (Variables|Default|GetObjectName)) false false)
    (Variables|Default|SetOverlappingPlayer false)))

(fn ConstructionScript)

(fn ScaleObject
  (params (DeltaSeconds :type Float%20%28double-precision%29) (Reset :type Boolean))
  (bind _icon (Variables|Default|GetIcon))
  (Transformation|SetRelativeScale3D _icon (Math|Interpolation|VInterpTo (Variables|/Script/Engine.SceneComponent|GetRelativeScale3D _icon) (Variables|Default|GettargetScaleVector) DeltaSeconds (LocalVariables|GetInterpSpeed))))

(fn Interact
  (params (InteractingActor :type Actor%20Object%20Reference))
  (Development|PrintString (Utilities|GetDisplayName InteractingActor) false)
  (Utilities|Casting|CastToBP_PlayerHero InteractingActor
    (:then
      (for _array_element (Class|PrimitiveComponent|GetOverlappingComponents (Variables|Default|GetCollision%20Mesh))
        (Development|PrintString (Utilities|String|Append "Overlapping: " (Utilities|GetDisplayName _array_element)) false)
        (if (Utilities|Enum|Equal(Enum) (Utilities|GetDisplayName _array_element) (LocalVariables|GetstringPlayerHeroCollisionBox))
          (LocalVariables|SetboolCloseEnough true)
          (else
            (Development|PrintString "Not close enough yet" false))))
      (if (LocalVariables|GetboolCloseEnough)
        (Development|PrintString (Utilities|String|Append (Utilities|String|Append (Utilities|String|Append (Utilities|String|Append "Clicked on " (Variables|Default|GetObjectName)) " while ") (Utilities|GetDisplayName InteractingActor)) " is within range") false)
        (if (Variables|Default|GethasDialogueTree)
          (CallFunction|ChooseAppropriateDialogueTree)
          (Default|BeginDialogue (Variables|Default|GetDialogueTree)))))
    (:CastFailed
      (Development|PrintString "Not in Range" false))))

(fn ChooseAppropriateDialogueTree
  (bind _returnvalue (Actor|GetComponentsByClass "/Game/TTRPG/Blueprints/DialogueTree.DialogueTree_C"))
  (bind _output (Utilities|Array|Get(acopy) _returnvalue))
  (Utilities|String|LogString "Beginning Dialougue Tree Choices")
  (bind _asttrpg_base (Utilities|Casting|CastToTTRPG_Base (Game|GetGameMode))
    (:then
      (LocalVariables|SetlocalCurrentTimeOfDay (Variables|/Game/TTRPG/TTRPG_Base.TTRPG_Base_C|GetCurrentTimeOfDay _asttrpg_base))
      (if (>= (Utilities|Array|Length _returnvalue) 2)
        (Variables|Default|SetDialogueTree _output)
        (for _array_element _returnvalue
          (if (Variables|/Game/TTRPG/Blueprints/DialogueTree.DialogueTree_C|Getactive _array_element) ; If the current Element is active continue
            (if (Variables|/Game/TTRPG/Blueprints/DialogueTree.DialogueTree_C|GetboolActiveQuest _array_element) ; If the element requires an active quest
              ;[1 1 1] Quest Requirements
              (bind _asttrpg_base_2 (Utilities|Casting|CastToTTRPG_Base (Game|GetGameMode)))
              (for _array_element_2 (Variables|/Game/TTRPG/Blueprints/Code-Implimented-Blueprints/BP_QuestController.BP_QuestController_C|GetcurrentQuests (Variables|/Game/TTRPG/TTRPG_Base.TTRPG_Base_C|GetQuestController _asttrpg_base_2))
                (if (not (.Completed (Utilities|Struct|BreakQuest _array_element_2))) ; If a quest is completed, skip it
                  (if (Utilities|Enum|Equal(Enum) (.InternalQuestName (Utilities|Struct|BreakQuest _array_element_2)) (Variables|/Game/TTRPG/Blueprints/DialogueTree.DialogueTree_C|GetinternalQuestName _array_element))
                    (if (Utilities|Array|IsNotEmpty (Variables|/Game/TTRPG/Blueprints/DialogueTree.DialogueTree_C|GetrequiredQuestStep _array_element))
                      (if (Utilities|Array|ContainsItem (Variables|/Game/TTRPG/Blueprints/DialogueTree.DialogueTree_C|GetrequiredQuestStep _array_element) (.CurrentStep (Utilities|Struct|BreakQuest _array_element_2)))
                        (LocalVariables|SetboolQuestDialogue true :!label _label)
                        (Variables|Default|SetDialogueTree _array_element))
                      (else
                        (goto _label))))))
              (elif (not (LocalVariables|GetboolQuestDialogue)) ; If we have already found a dialogue tree that requires a quest that we have, then do not display non-quest related Dialogue Trees
                (if (Utilities|Array|IsNotEmpty (Variables|/Game/TTRPG/Blueprints/DialogueTree.DialogueTree_C|GettimeOfDay _array_element)) ; if the current Element has Time of Day check for matching Time of Day. If not continue to priority
                  (Development|PrintString "Time of Day is not empty")
                  (if (Utilities|Array|ContainsItem (Variables|/Game/TTRPG/Blueprints/DialogueTree.DialogueTree_C|GettimeOfDay _array_element) (LocalVariables|GetlocalCurrentTimeOfDay)) ; If Dialogue Tree has active time of day matching current time of day, then proceed to priorty. Otherwise move on to next element
                    (Development|PrintString "Current Time Equals Element TIme of day")
                    (if (< (Variables|/Game/TTRPG/Blueprints/DialogueTree.DialogueTree_C|GetPriority _array_element) (Variables|/Game/TTRPG/Blueprints/DialogueTree.DialogueTree_C|GetPriority (Variables|Default|GetDialogueTree))) :!label _label_2 ; If current priority is 'lower' than the element priority set to new Dialogue Tree. Otherwise go to next element
                      (Variables|Default|SetDialogueTree _array_element)
                      (Development|PrintString "Dialogue Tree Set"))
                    (else
                      (Development|PrintString "Time of Day is NOT included")))
                  (else
                    (goto _label_2)))))))
        (Development|PrintString (Utilities|String|Append "Dialogue Tree to display is: " (Variables|/Game/TTRPG/Blueprints/DialogueTree.DialogueTree_C|GetDisplay%20Name (Variables|Default|GetDialogueTree))))
        (return)
        (else
          (Variables|Default|SetDialogueTree _output))))
    (:CastFailed
      (Utilities|String|LogString "Failed Game Mode Cast in Interactable Object")
      (return))))

(fn VerifyQuestRequirement
  (bind _requiredqueststep (Variables|Default|GetrequiredQuestStep))
  (bind _asttrpg_base (Utilities|Casting|CastToTTRPG_Base (Game|GetGameMode))
    (:then
      (for _array_element (Variables|/Game/TTRPG/Blueprints/Code-Implimented-Blueprints/BP_QuestController.BP_QuestController_C|GetcurrentQuests (Variables|/Game/TTRPG/TTRPG_Base.TTRPG_Base_C|GetQuestController _asttrpg_base))
        (if (Utilities|Enum|Equal(Enum) (.InternalQuestName (Utilities|Struct|BreakQuest _array_element)) (Variables|Default|GetrequiredQuestInternalName)) ; Only return true if the required quest is active
          (if (not (.Completed (Utilities|Struct|BreakQuest _array_element))) ; Only return true if the required quest is not yet completed
            (if (Utilities|Array|IsNotEmpty _requiredqueststep)
              (if (Utilities|Array|ContainsItem _requiredqueststep (.CurrentStep (Utilities|Struct|BreakQuest _array_element))) ; Only return true if the required quest in the allowed step/steps
                (LocalVariables|SettempReturnBool true :!label _label))
              (else
                (goto _label))))))
      (return (LocalVariables|GettempReturnBool)))
    (:CastFailed
      (return false))))