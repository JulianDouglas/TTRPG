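; BP_PlayerHero is the player's hero pawn in a TTRPG game, handling camera zoom, interactable reveal and terrain-based speed.
; Tick eases spring arm length toward clamped zoom requests or back to its default, with zoom taking priority.
; AreaReveal overlaps scale InteractableObjects up and down.
; Capsule overlaps tell the controller to end moves at a PlayerMoveBox, or set speed from a NavModifierVolume's area class, restoring it on exit.
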(event OnComponentBeginOverlap(AreaReveal)
  (params (OverlappedComponent :type Primitive%20Component%20Object%20Reference) (OtherActor :type Actor%20Object%20Reference) (OtherComp :type Primitive%20Component%20Object%20Reference) (OtherBodyIndex :type Integer) (bFromSweep :type Boolean) (SweepResult :type Hit%20Result%20Structure%20%28by%20ref%29))
  (Development|PrintString (Utilities|GetDisplayName OverlappedComponent) false false)
  (bind _asinteractable_object (Utilities|Casting|CastToInteractableObject OtherActor))
  (Default|ScaleInteractableObject _asinteractable_object))

(event OnComponentEndOverlap(AreaReveal)
  (params (OverlappedComponent :type Primitive%20Component%20Object%20Reference) (OtherActor :type Actor%20Object%20Reference) (OtherComp :type Primitive%20Component%20Object%20Reference) (OtherBodyIndex :type Integer))
  (bind _asinteractable_object (Utilities|Casting|CastToInteractableObject OtherActor))
  (Default|DownScaleInteractableObject _asinteractable_object))

(event OnComponentEndOverlap(CapsuleComponent)
  (params (OverlappedComponent :type Primitive%20Component%20Object%20Reference) (OtherActor :type Actor%20Object%20Reference) (OtherComp :type Primitive%20Component%20Object%20Reference) (OtherBodyIndex :type Integer))
  (Utilities|Casting|CastToNavModifierVolume OtherActor)
  (Development|PrintString "Cast To Nav Mod Volume Succeeded" false false)
  (CallFunction|ResetPlayerSpeed))

(event OnComponentBeginOverlap(CapsuleComponent)
  (params (OverlappedComponent :type Primitive%20Component%20Object%20Reference) (OtherActor :type Actor%20Object%20Reference) (OtherComp :type Primitive%20Component%20Object%20Reference) (OtherBodyIndex :type Integer) (bFromSweep :type Boolean) (SweepResult :type Hit%20Result%20Structure%20%28by%20ref%29))
  (Development|PrintString (Utilities|GetClassDisplayName (Utilities|GetClass OtherActor)) true false)
  (if (Utilities|String|Contains (Utilities|GetDisplayName OtherComp) "PlayerMoveBox")
    (Development|PrintString "Arrived" true false)
    (bind _asttrpg_base_controller (Utilities|Casting|CastToTTRPG_BaseController (Pawn|GetController)))
    (Default|EndMoveto _asttrpg_base_controller))
  (bind _asnav_modifier_volume (Utilities|Casting|CastToNavModifierVolume OtherActor)
    (:then
      (Development|PrintString "Cast To Nav Mod Volume Succeeded" false false)
      (CallFunction|AdjustPlayerSpeed _asnav_modifier_volume))
    (:CastFailed
      (Development|PrintString "Cast to Nav Mod Volume Failed" false false))))

(event Custom|AdjustSpringArm
  (params (AdjustmentValue :type Float%20%28double-precision%29))
  (Variables|Default|Setfloat_tempSpringLength (Math|Float|Clamp(Float) (+ (* AdjustmentValue -1e+03) (Variables|/Script/Engine.SpringArmComponent|GetTargetArmLength (Variables|Camera|GetSpringArm))) 2e+03 4e+03))
  (Variables|Default|Setbool_moveSpring true))

(event EventTick
  (params (DeltaSeconds :type Float%20%28single-precision%29))
  (if (Variables|Default|Getbool_moveSpring)
    (Variables|Default|Setbool_resetCamera false)
    (CallFunction|SpringInterp DeltaSeconds)
    (elif (Variables|Default|Getbool_resetCamera)
      (CallFunction|CameraResetInterp DeltaSeconds))))

(fn ConstructionScript)

(fn ResetSpringArm
  (Variables|Default|Setbool_resetCamera true))

(fn SpringInterp
  (params (DeltaTime :type Float%20%28double-precision%29))
  (bind _springarm (Variables|Camera|GetSpringArm))
  (bind _float_tempspringlength (Variables|Default|Getfloat_tempSpringLength))
  (bind _returnvalue (Math|Float|Round _float_tempspringlength))
  (bind _returnvalue_2 (Math|Conversions|ToFloat(Integer) _returnvalue))
  (Development|PrintString (Utilities|String|Append "Starting SpringCompare: " (Utilities|String|Append (Utilities|String|ToString(Float) (Math|Conversions|ToFloat(Integer) (Math|Float|Round (Variables|/Script/Engine.SpringArmComponent|GetTargetArmLength _springarm)))) (Utilities|String|ToString(Float) _returnvalue_2))) false false)
  (Math|Float|CompareFloat (Math|Conversions|ToFloat(Integer) (Math|Float|Round (Variables|/Script/Engine.SpringArmComponent|GetTargetArmLength _springarm))) _returnvalue_2
    (:>
      (Variables|/Script/Engine.SpringArmComponent|SetTargetArmLength _springarm (Math|Interpolation|FInterptoConstant (Variables|/Script/Engine.SpringArmComponent|GetTargetArmLength _springarm) _float_tempspringlength DeltaTime 1.5e+03) :!label _label))
    (:==
      (Development|PrintString "Resetting Temp Spring Length" false false)
      (Variables|Default|Setbool_moveSpring false))
    (:<
      (goto _label))))

(fn CameraResetInterp
  (params (DeltaTime :type Float%20%28double-precision%29))
  (bind _springarm (Variables|Camera|GetSpringArm))
  (bind _int_defaultspringarm (Variables|Default|Getint_DefaultSpringArm))
  (bind _returnvalue (Math|Float|Round _int_defaultspringarm))
  (bind _returnvalue_2 (Math|Conversions|ToFloat(Integer) _returnvalue))
  (Development|PrintString (Utilities|String|Append "Starting Camera Reset Compare" (Utilities|String|Append (Utilities|String|ToString(Float) (Math|Conversions|ToFloat(Integer) (Math|Float|Round (Variables|/Script/Engine.SpringArmComponent|GetTargetArmLength _springarm)))) (Utilities|String|ToString(Float) _returnvalue_2))) false false)
  (Math|Float|CompareFloat (Math|Conversions|ToFloat(Integer) (Math|Float|Round (Variables|/Script/Engine.SpringArmComponent|GetTargetArmLength _springarm))) (+ _returnvalue_2 1e+01)
    (:>
      (Variables|/Script/Engine.SpringArmComponent|SetTargetArmLength _springarm (Math|Interpolation|FInterptoConstant (Math|Conversions|ToFloat(Integer) (Math|Float|Round (Variables|/Script/Engine.SpringArmComponent|GetTargetArmLength _springarm))) _returnvalue_2 DeltaTime 1e+03)))
    (:==
      (Development|PrintString "Resetting Arm Length" false false :!label _label)
      (Variables|Default|Setbool_resetCamera false)
      (Variables|/Script/Engine.SpringArmComponent|SetTargetArmLength _springarm _returnvalue_2))
    (:<
      (goto _label))))

(fn AdjustPlayerSpeed
  (params (Nav%20Volume :type Nav%20Modifier%20Volume%20Object%20Reference))
  (Development|PrintString "Adjusting Player Speed")
  (bind _asnav_area_ttrpgbase (Utilities|Casting|CastToNavArea_TTRPGBaseClass (Variables|/Script/NavigationSystem.NavModifierVolume|GetAreaClass Nav%20Volume)))
  (bind _asttrpg_base_controller (Utilities|Casting|CastToTTRPG_BaseController (Pawn|GetController)))
  (Default|SetPlayerSpeed _asttrpg_base_controller (Utilities|GetClassDefaults _asnav_area_ttrpgbase)))

(fn ResetPlayerSpeed
  (Development|PrintString "Resetting Player Speed")
  (bind _asttrpg_base_controller (Utilities|Casting|CastToTTRPG_BaseController (Pawn|GetController)))
  (Default|SetPlayerSpeed _asttrpg_base_controller 2e+02))