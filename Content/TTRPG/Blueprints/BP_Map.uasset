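; BP_Map is a tabletop RPG map actor with a FogOfWar component whose material density can be changed.
; The construction script gives FogOfWar a dynamic material instance on its first material slot.
; The AdjustDensity event prints a debug message and sets the Density parameter to a fixed offset plus that parameter's custom primitive data index, rather than its current value.
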(event Custom|AdjustDensity
  (bind _fogofwar (Variables|Default|GetFogOfWar))
  (Development|PrintText "Adjusting Density")
  (Rendering|Material|SetScalarParameterValueonMaterials _fogofwar "Density" (+ 0.5 (Math|Conversions|ToFloat(Integer) (Class|PrimitiveComponent|GetCustomPrimitiveDataIndexforScalarParameter _fogofwar "Density")))))

(event EventBeginPlay)

(event Collision|EventActorBeginOverlap
  (params (OtherActor :type Actor%20Object%20Reference)))

(event EventTick
  (params (DeltaSeconds :type Float%20%28single-precision%29)))

(fn ConstructionScript
  (bind _returnvalue (Rendering|Material|CreateDynamicMaterialInstance (Variables|Default|GetFogOfWar) 0 0 "None" :!class /Script/Engine.PrimitiveComponent))
  (Rendering|Material|SetMaterial (Variables|Default|GetFogOfWar) 0 _returnvalue))